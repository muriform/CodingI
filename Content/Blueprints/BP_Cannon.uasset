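; BP_Cannon is a cannon actor that automatically fires a cannonball every second once play begins.
; BeginPlay runs an endless Delay loop that calls the FireCannon event.
; FireCannon spawns a BP_Cannonball at the Spawnpoint transform and launches its Cube with a single mass-independent AddForce along the Spawnpoint's forward vector.
; It also prints a firing message with the running shot count, then increments that count.
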(event Custom|FireCannon
  (Development|PrintText (Utilities|Text|FormatText "Firing cannonball {shotcount}!" (Variables|Default|GetShotcount)))
  (bind _returnvalue (Game|SpawnActorfromClass "/Game/Blueprints/BP_Cannonball.BP_Cannonball_C" (Transformation|GetWorldTransform (Variables|Default|GetSpawnpoint)) "Undefined" "MultiplyWithRoot" 0 0))
  (Physics|AddForce (Variables|/Game/Blueprints/BP_Cannonball.BP_Cannonball_C|GetCube _returnvalue) (* (Math|Vector|GetForwardVector (Variables|Default|GetSpawnpoint)) 1e+05) "None" true)
  (Math|Integer|IncrementInt (Variables|Default|GetShotcount)))

(event EventBeginPlay
  (Utilities|FlowControl|Delay 1.0 :!label _label)
  (CallFunction|FireCannon)
  (goto _label))

(fn ConstructionScript)