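; BP_RockSpawner is a pickup item, described in its messages as a rock planter, that the third-person character can carry and use.
; On overlap it caches the character and calls TrytoPickupItem, while its Pickup event snaps it to the player mesh's right-hand grip socket.
; PrimaryAction spawns a BP_Tree, not a rock, at the item's transform, and Drop destroys the item.
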(event EventBeginPlay)

(event Collision|EventActorBeginOverlap
  (params (OtherActor :type Actor%20Object%20Reference))
  (bind _asbp_third_person_character (Utilities|Casting|CastToBP_ThirdPersonCharacter OtherActor))
  (Variables|Components|SetPlayer _asbp_third_person_character)
  (Default|TrytoPickupItem _asbp_third_person_character self))

(event EventTick
  (params (DeltaSeconds :type Float%20%28single-precision%29)))

(event EventPickup
  (Development|PrintText "The rock planter is getting picked up!")
  (Transformation|AttachComponentToComponent (Variables|/Script/Engine.Character|GetMesh (Variables|Components|GetPlayer)) "HandGrip_R" "SnapToTarget" "SnapToTarget" "KeepRelative" true))

(event EventPrimaryAction
  (Development|PrintText "Let's plant some rocks!")
  (Game|SpawnActorfromClass "/Game/Blueprints/BP_Tree.BP_Tree_C" (Transformation|GetActorTransform) "Undefined" "MultiplyWithRoot" 0 0))

(event EventDrop
  (Development|PrintText "The rock planter has been dropped!")
  (Actor|DestroyActor))

(fn ConstructionScript)