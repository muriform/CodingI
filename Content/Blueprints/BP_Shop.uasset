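; BP_Shop is a shop actor for selling fish for credit, displayed as Bridges.
; Any actor overlap casts player 0 to BP_ThirdPersonCharacter and reads its fish and credit through getter calls.
; With fish available, it decrements the fish value, increments credit and prints the totals, with no explicit setter call back to the character.
; The shop's own GetTotalfish and GetCredit functions are empty stubs.
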(event EventBeginPlay)

(event EventTick
  (params (DeltaSeconds :type Float%20%28single-precision%29)))

(event Collision|EventActorBeginOverlap
  (params (OtherActor :type Actor%20Object%20Reference))
  ;[0.15 0.15 0.15 0.5] Selling Fish
  (bind _asbp_third_person_character (Utilities|Casting|CastToBP_ThirdPersonCharacter (Game|GetPlayerCharacter 0))
    (:then
      (Default|GetTotalfish _asbp_third_person_character (Variables|Default|GetTotalFish))
      (if (> (Variables|Default|GetTotalFish) 0)
        (Default|GetCredit _asbp_third_person_character (Variables|Default|GetCredit))
        (Math|Integer|DecrementInt (Variables|Default|GetTotalFish)
          (:%20%20
            (Math|Integer|IncrementInt (Variables|Default|GetCredit)
              (:%20%20
                (Development|PrintText (Utilities|Text|FormatText "You sold a fish! You now have {Credit} Bridges and {Total Fish} Fish!" (Variables|Default|GetCredit) (Variables|Default|GetTotalFish)))))))
        (else
          (Development|PrintText "You have no fish!"))))
    (:CastFailed
      (Development|PrintText "CAST FAILED"))))

(fn ConstructionScript)

(fn GetTotalfish
  (params (Amount :type Integer)))

(fn GetCredit
  (params (Amount :type Integer)))