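; BP_DialogueManager shows dialogue lines one at a time, cycling through a Dialogue text array.
; BeginPlay creates and stores a W_Dialogue widget.
; Each DisplayNextLine call prints the current line, writes it to the widget, and adds it to the viewport until a short delay removes it.
; A Sequence advances the index without waiting for that delay, and the index wraps to the start once past the last line.
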(event Custom|DisplayNextLine
  (bind _dialoguewidget (Variables|Default|GetDialogueWidget))
  (if (>= (Variables|Default|GetIndex) (Utilities|Array|Length (Variables|Default|GetDialogue)))
    (Variables|Default|SetIndex 0))
  (Development|PrintText (Utilities|Array|Get(acopy) (Variables|Default|GetDialogue) (Variables|Default|GetIndex)) true true "(R=0.000000,G=0.283290,B=1.000000,A=1.000000)" 1e+01)
  (Rendering|Components|TextRender|SetText (Variables|/Game/Widgets/W_Dialogue.W_Dialogue_C|GetTextBlock_0 _dialoguewidget) (Utilities|Array|Get(acopy) (Variables|Default|GetDialogue) (Variables|Default|GetIndex)))
  (Utilities|FlowControl|Sequence
    (:then_0
      (UserInterface|Viewport|AddtoViewport _dialoguewidget 0)
      (Utilities|FlowControl|Delay 5.0)
      (Widget|RemovefromParent _dialoguewidget))
    (:then_1
      (Math|Integer|IncrementInt (Variables|Default|GetIndex)) ; ++ to add 1 to index
    )))

(event EventBeginPlay
  (bind _returnvalue (UserInterface|CreateWidget "/Game/Widgets/W_Dialogue.W_Dialogue_C"))
  (Variables|Default|SetDialogueWidget _returnvalue))

(fn ConstructionScript)